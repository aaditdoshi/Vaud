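; Mantle component that lifts the owning player character onto ledges, driven by a Start/Climb/Push state machine on Tick.
; Start sphere-traces forward for the wall and downward for the ledge, triggering a climb when the ledge is no higher than the capsule top.
; Climb disables input, switches to Flying and lerps the character above the ledge with sweep.
; Push restores input and the saved movement mode, without applying forward motion.
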(event Custom|Climb%20Ledge
  (params (DeltaSeconds :type Float%20%28single-precision%29))
  (bind _walllocation (Variables|Default|GetWallLocation))
  (bind _asplayer_game_character (Utilities|Casting|CastToPlayerGameCharacter (Components|GetOwner)))
  (Components|Movement|StopMovementImmediately (Variables|/Script/Engine.Character|GetCharacterMovement _asplayer_game_character))
  (Input|DisableInput _asplayer_game_character 0)
  (Utilities|FlowControl|Sequence
    (:then_0
      (Utilities|FlowControl|DoOnce false :!label _label
        (:Completed
          (Variables|Default|SetPreviousMovementMode (Variables|/Script/Engine.CharacterMovementComponent|GetMovementMode (Variables|/Script/Engine.Character|GetCharacterMovement _asplayer_game_character))))))
    (:then_1
      (Pawn|Components|CharacterMovement|SetMovementMode (Variables|/Script/Engine.Character|GetCharacterMovement _asplayer_game_character) "MOVE_Flying" 0)
      (Variables|Default|SetDistanceToPoint (Math|Vector|VectorLength (- (Math|Vector|MakeVector (.x _walllocation) (.y _walllocation) (+ (* (.OutHalfHeight (Components|Capsule|GetScaledCapsuleSize (Variables|/Script/Engine.Character|GetCapsuleComponent _asplayer_game_character))) 2.0) (.z (Variables|Default|GetHeightLocation)))) (Transformation|GetActorLocation _asplayer_game_character))))
      (Class|KismetMathLibrary|VectorSpringInterp "0, 0, 0" "0, 0, 0" (Variables|Default|GetClimbState) 0.9 2.0 DeltaSeconds 1.0)
      (Transformation|SetActorLocation _asplayer_game_character (Math|Vector|Lerp(Vector) (Transformation|GetActorLocation _asplayer_game_character) (Math|Vector|MakeVector (.x _walllocation) (.y _walllocation) (+ (* (.OutHalfHeight (Components|Capsule|GetScaledCapsuleSize (Variables|/Script/Engine.Character|GetCapsuleComponent _asplayer_game_character))) 2.0) (.z (Variables|Default|GetHeightLocation)))) 0.5) true false)
      (Development|PrintString (Utilities|String|ToString(Float) (Variables|Default|GetDistanceToPoint)))
      (if (<= (Variables|Default|GetDistanceToPoint) 1e+01)
        (Variables|Default|SetCurrentState "Push")
        (goto _label Reset)))))

(event Custom|PushForward
  (bind _previousmovementmode (Variables|Default|GetPreviousMovementMode))
  (bind _asplayer_game_character (Utilities|Casting|CastToPlayerGameCharacter (Components|GetOwner)))
  (Input|EnableInput _asplayer_game_character 0)
  (Pawn|Components|CharacterMovement|SetMovementMode (Variables|/Script/Engine.Character|GetCharacterMovement _asplayer_game_character) _previousmovementmode 0)
  (Development|PrintString (Utilities|String|EnumtoString _previousmovementmode))
  (Variables|Default|SetCurrentState "Start"))

(event EventBeginPlay)

(event EventTick
  (params (DeltaSeconds :type Float%20%28single-precision%29))
  (switch Utilities|FlowControl|Switch|SwitchonFMantleState (Variables|Default|GetCurrentState)
    (:Start
      (CallFunction|ForwardTrace)
      (bind _returnvalue (CallFunction|HeightTrace))
      (if _returnvalue
        (Variables|Default|SetCurrentState "Climb")))
    (:Climb
      (CallFunction|ClimbLedge DeltaSeconds))
    (:Push
      (CallFunction|PushForward))))

(fn ForwardTrace
  (bind _returnvalue (Components|GetOwner))
  (bind _mantledistancecheck (Variables|Default|GetMantleDistanceCheck))
  (bind _returnvalue_2 (Transformation|GetActorLocation _returnvalue))
  (bind _returnvalue_3 (Transformation|GetActorForwardVector _returnvalue))
  (bind _returnvalue_4 (* (Math|Vector|MakeVector (.x _returnvalue_3) (.y _returnvalue_3) 0.0) _mantledistancecheck))
  (bind (_outhit _returnvalue_5) (Collision|SphereTraceByChannel _returnvalue_2 (+ _returnvalue_2 (Math|Vector|MakeVector (.x _returnvalue_4) (.y _returnvalue_4) (.z _returnvalue_3))) 2e+01 "TraceTypeQuery3" false 0 "None"))
  (if _returnvalue_5
    (Variables|Default|SetWallLocation (.Location (Collision|BreakHitResult _outhit)))
    (Variables|Default|SetWallNormal (.Normal (Collision|BreakHitResult _outhit)))))

(fn HeightTrace
  (bind _returnvalue (Components|GetOwner))
  (bind _returnvalue_2 (Components|GetOwner))
  (bind _mantledistancecheck (Variables|Default|GetMantleDistanceCheck))
  (bind _returnvalue_3 (Transformation|GetActorForwardVector _returnvalue))
  (bind _returnvalue_4 (Transformation|GetActorLocation _returnvalue))
  (bind _returnvalue_5 (* _returnvalue_3 _mantledistancecheck))
  (bind _returnvalue_6 (+ _returnvalue_4 _returnvalue_5))
  (bind (_outhit _returnvalue_7) (Collision|SphereTraceByChannel (+ _returnvalue_6 (Math|Vector|MakeVector 0.0 0.0 (Variables|Default|GetMantleHeightCheck))) _returnvalue_6 2e+01 "TraceTypeQuery3" false 0 "None"))
  (if _returnvalue_7
    (bind _output_get (Variables|Default|SetHeightLocation (.Location (Collision|BreakHitResult _outhit))))
    (bind _asbp_player_game_character (Utilities|Casting|CastToBP_PlayerGameCharacter _returnvalue_2))
    (Development|PrintString (Utilities|String|ToString(Float) (- (.z _output_get) (+ (Components|Capsule|GetScaledCapsuleHalfHeight (Variables|/Script/Engine.Character|GetCapsuleComponent _asbp_player_game_character)) (.z (Transformation|GetActorLocation _returnvalue_2))))))
    (if (<= (- (.z _output_get) (+ (Components|Capsule|GetScaledCapsuleHalfHeight (Variables|/Script/Engine.Character|GetCapsuleComponent _asbp_player_game_character)) (.z (Transformation|GetActorLocation _returnvalue_2)))) 0.0)
      (return true)
      (else
        (return false)))))