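; BP_ArcheryCharacter is a player character Blueprint that wires input to a weapon component and wall running.
; On BeginPlay it creates a crosshair widget for the first player controller and adds it to the viewport.
; Fire press and release forward to the WeaponComponent's fire start and stop calls after a validity check.
; Jump press and release activate and deactivate the WallRun component, with no jump call in this graph.
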(event EventBeginPlay
  (|CallParentFunction)
  (bind _returnvalue (UserInterface|CreateWidget "/Game/Users/Aadit/HUD/Widget_Crosshair.Widget_Crosshair_C" (Game|GetPlayerController 0)))
  (UserInterface|Viewport|AddtoViewport _returnvalue 0))

(event Collision|EventActorBeginOverlap
  (params (OtherActor :type Actor%20Object%20Reference))
  (|CallParentFunction OtherActor) ; This node is disabled and will not be called.\nDrag off pins to build functionality.
)

(event EventTick
  (params (DeltaSeconds :type Float%20%28single-precision%29))
  (|CallParentFunction DeltaSeconds) ; This node is disabled and will not be called.\nDrag off pins to build functionality.
)

(event Input|ActionEvents|InputActionFire
  (params (Key :type Key%20Structure))
  (bind _weaponcomponent (Variables|Default|GetWeaponComponent))
  (bind _weaponcomponent_2 (Variables|Default|GetWeaponComponent))
  (:Pressed
    (Utilities|IsValid _weaponcomponent
      (:Is%20Valid
        (Class|WeaponComponent|OnFire _weaponcomponent))))
  (:Released
    (Utilities|IsValid _weaponcomponent_2
      (:Is%20Valid
        (Class|WeaponComponent|OnFireStopped _weaponcomponent_2)))))

(event Input|ActionEvents|InputActionJump
  (params (Key :type Key%20Structure))
  (bind _wallrun (Variables|Default|GetWallRun))
  (:Pressed
    (Components|Activation|Activate _wallrun false))
  (:Released
    (Components|Activation|Deactivate _wallrun)))

(fn ConstructionScript
  (|CallParentFunction))