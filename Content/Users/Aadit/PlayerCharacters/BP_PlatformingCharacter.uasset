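; BP_PlatformingCharacter is a player character Blueprint that adds double jump and wall run control to the Jump input.
; Holding Jump keeps the WallRun component active, and releasing it deactivates the component.
; A DoN counter limits presses to two, launching the character upward at DoubleJumpVelocity on the second, and resets on landing.
; The first press triggers no launch in this graph.
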(event EventBeginPlay
  (|CallParentFunction) ; This node is disabled and will not be called.\nDrag off pins to build functionality.
)

(event Collision|EventActorBeginOverlap
  (params (OtherActor :type Actor%20Object%20Reference))
  (|CallParentFunction OtherActor) ; This node is disabled and will not be called.\nDrag off pins to build functionality.
)

(event EventTick
  (params (DeltaSeconds :type Float%20%28single-precision%29))
  (|CallParentFunction DeltaSeconds) ; This node is disabled and will not be called.\nDrag off pins to build functionality.
)

(event EventOnLanded
  (params (Hit :type Hit%20Result%20Structure%20%28by%20ref%29))
  (Utilities|FlowControl|DoN 2) ; enters at Reset
)

(event Input|ActionEvents|InputActionJump
  (params (Key :type Key%20Structure))
  (:Pressed
    (Components|Activation|Activate (Variables|Default|GetWallRun) false)
    (bind _counter (Utilities|FlowControl|DoN 2)
      (:Exit
        (switch int _counter
          (:2
            (Character|LaunchCharacter (Math|Vector|MakeVector 0.0 0.0 (Variables|Default|GetDoubleJumpVelocity)) false true))))))
  (:Released
    (Components|Activation|Deactivate (Variables|Default|GetWallRun))))

(fn ConstructionScript
  (|CallParentFunction))