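; BP_BaseBow is a base bow weapon that attaches to the player's first-person mesh when equipped.
; Setup aligns the bow's Handle socket to BowSocket, then spawns an ArrowClass actor and copies its mesh onto an arrow component attached at ArrowSocket.
; Fire press and release toggle a holding flag, with Tick calling DrawBow while held and not reloading.
; DrawBow and ReleaseBow are stubs, so no draw progression or shooting happens here.
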(event Custom|Draw%20Bow
  (if (< (Variables|Default|GetDrawBowPercent) 1.0)
    _))

(event Custom|Release%20Bow)

(event EventBeginPlay)

(event Collision|EventActorBeginOverlap
  (params (OtherActor :type Actor%20Object%20Reference)))

(event EventOnFireStopped
  (Variables|Default|SetIsHolding false)
  (CallFunction|ReleaseBow))

(event EventTick
  (params (DeltaSeconds :type Float%20%28single-precision%29))
  (bind _returnvalue (Class|Weapon|IsReloading))
  (if (and (not _returnvalue) (Variables|Default|GetIsHolding))
    (CallFunction|DrawBow)))

(event EventOnEquipped
  (bind _asbp_player_game_character (Utilities|Casting|CastToBP_PlayerGameCharacter (Components|GetOwner)))
  (CallFunction|SetUpBow (Variables|/Script/Vaudeville.PlayerGameCharacter|GetFirstPersonMesh _asbp_player_game_character))
  (CallFunction|SetUpArrow (Variables|/Script/Vaudeville.PlayerGameCharacter|GetFirstPersonMesh _asbp_player_game_character)))

(event EventOnFire
  (Variables|Default|SetIsHolding true))

(fn ConstructionScript)

(fn SetUpBow
  (params (FirsPersonMesh :type Scene%20Component%20Object%20Reference))
  ;[1 1 1] Set Up Bow
  (Transformation|SetActorTransform self (Transformation|GetSocketTransform FirsPersonMesh "BowSocket" "RTS_World") false true)
  (Transformation|AttachComponentToComponent self FirsPersonMesh "BowSocket" "KeepWorld" "KeepWorld" "KeepWorld" true)
  (Transformation|AddActorLocalOffset self (* (.location (Transformation|GetSocketTransform (Variables|Default|GetWeaponStaticMesh) "Handle" "RTS_Actor")) -1.0) false false))

(fn SetUpArrow
  (params (FirstPersonMesh :type Scene%20Component%20Object%20Reference))
  (bind _returnvalue (Game|SpawnActorfromClass (Variables|Default|GetArrowClass) (Transformation|GetSocketTransform FirstPersonMesh "ArrowSocket" "RTS_World") "Undefined" 0 0))
  (Components|StaticMesh|SetStaticMesh (Variables|Default|GetArrowMeshComponent) (Variables|/Script/Engine.StaticMeshComponent|GetStaticMesh (Variables|/Game/Users/Aadit/Weapons/Bow/BP_BaseArrow.BP_BaseArrow_C|GetArrowMesh _returnvalue)))
  (Transformation|AttachComponentToComponent (Variables|Default|GetArrowMeshComponent) FirstPersonMesh "ArrowSocket" "SnapToTarget" "SnapToTarget" "SnapToTarget" true))