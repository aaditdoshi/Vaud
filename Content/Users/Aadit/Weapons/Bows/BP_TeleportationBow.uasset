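; BP_TeleportationBow is a bow weapon variant that previews where its arrow will land while held.
; Each Tick while IsHolding, it predicts a projectile path from the owning player's first-person camera.
; Launch speed scales with draw time between the arrow class's default minimum and maximum speeds.
; A debug sphere marks the predicted endpoint; firing and teleport logic are absent from this graph.
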(event EventBeginPlay
  (|CallParentFunction) ; This node is disabled and will not be called.\nDrag off pins to build functionality.
)

(event Collision|EventActorBeginOverlap
  (params (OtherActor :type Actor%20Object%20Reference))
  (|CallParentFunction OtherActor) ; This node is disabled and will not be called.\nDrag off pins to build functionality.
)

(event EventTick
  (params (DeltaSeconds :type Float%20%28single-precision%29))
  (bind _arrowclass (Variables|Default|GetArrowClass))
  (bind _ammodata (Utilities|GetClassDefaults _arrowclass))
  (|CallParentFunction DeltaSeconds)
  (if (Variables|Default|GetIsHolding)
    (bind _asbp_player_game_character (Utilities|Casting|CastToBP_PlayerGameCharacter (Components|GetOwner)))
    (bind _outlasttracedestination (Class|GameplayStatics|BlueprintPredictProjectilePathbyTraceChannel (+ (.WorldLocatiion (Default|GetFirstPersonCameraOrientation _asbp_player_game_character)) (* (.ForwardVector (Default|GetFirstPersonCameraOrientation _asbp_player_game_character)) (Variables|Default|GetProjectileSpawnOffset))) (* (.ForwardVector (Default|GetFirstPersonCameraOrientation _asbp_player_game_character)) (Math|Float|MapRangeClamped (Math|Float|MapRangeClamped (Variables|Default|GetTenseTimer) 0.0 (Variables|Default|GetTimeTillFullyDrawn) 0.0 1.0) 0.0 1.0 (.minspeed _ammodata) (.maxspeed _ammodata))) true 1e+01 "ECC_GameTraceChannel1" false 0 "None"))
    (Rendering|Debug|DrawDebugSphere _outlasttracedestination 1e+02 12 "(R=1.000000,G=1.000000,B=1.000000,A=1.000000)" 0.5 5.0)))

(fn ConstructionScript
  (|CallParentFunction))