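; Tracer bow weapon that previews the arrow's predicted flight path while it is held.
; Each tick calls the parent logic, then predicts a projectile path from the owning player character's first-person camera.
; Launch speed scales with draw time between the arrow class's min and max speeds, with its fall speed as gravity override.
; The trajectory is rendered only as one-frame debug drawing from the prediction trace.
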(event Custom|DrawArrowTrajectory
  (bind _arrowclass (Variables|Default|GetArrowClass))
  (bind _ammodata (Utilities|GetClassDefaults _arrowclass))
  (if (Variables|Default|GetIsHolding)
    (bind _asbp_player_game_character (Utilities|Casting|CastToBP_PlayerGameCharacter (Components|GetOwner)))
    (Class|GameplayStatics|BlueprintPredictProjectilePathbyTraceChannel (.WorldLocatiion (Default|GetFirstPersonCameraOrientation _asbp_player_game_character)) (* (.ForwardVector (Default|GetFirstPersonCameraOrientation _asbp_player_game_character)) (Math|Float|MapRangeClamped (Math|Float|MapRangeClamped (Variables|Default|GetTenseTimer) 0.0 (Variables|Default|GetTimeTillFullyDrawn) 0.0 1.0) 0.0 1.0 (.minspeed _ammodata) (.maxspeed _ammodata))) true 1.0 "ECC_Visibility" false 0 "ForOneFrame" 5.0 3e+01 2.0 (.fallspeed _ammodata))))

(event EventBeginPlay
  (|CallParentFunction) ; This node is disabled and will not be called.\nDrag off pins to build functionality.
)

(event Collision|EventActorBeginOverlap
  (params (OtherActor :type Actor%20Object%20Reference))
  (|CallParentFunction OtherActor) ; This node is disabled and will not be called.\nDrag off pins to build functionality.
)

(event EventTick
  (params (DeltaSeconds :type Float%20%28single-precision%29))
  (|CallParentFunction DeltaSeconds)
  (CallFunction|DrawArrowTrajectory))

(fn ConstructionScript
  (|CallParentFunction))