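; Base bow arrow projectile that flies, then sticks into what it hits.
; Construction sets mesh, gravity and speed limits from AmmoData, scaling launch speed by DrawPercentage.
; The first overlap, ignoring the owner's owner, plays an impact sound, stops movement and trail particles, and attaches the arrow to the hit actor.
; Physics-simulating targets also get speed-scaled penetration and an impulse-like force at the arrow's location.
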(event OnComponentBeginOverlap(CollisionBox)
  (params (OverlappedComponent :type Primitive%20Component%20Object%20Reference) (OtherActor :type Actor%20Object%20Reference) (OtherComp :type Primitive%20Component%20Object%20Reference) (OtherBodyIndex :type Integer) (bFromSweep :type Boolean) (SweepResult :type Hit%20Result%20Structure%20%28by%20ref%29))
  (bind _projectilemovement (Variables|Default|GetProjectileMovement))
  (if (not (Variables|Default|GetHit))
    (if (!= OtherActor (Components|GetOwner (Components|GetOwner)))
      (Audio|PlaySoundatLocation "/Game/Users/Aadit/AudioEvents/Wav_WoodPenetrateImpact.Wav_WoodPenetrateImpact" (Transformation|GetActorLocation))
      (if (Physics|IsSimulatingPhysics OtherComp "None")
        (CallFunction|AddForcetoObject OtherComp))
      (Components|Movement|StopMovementImmediately _projectilemovement)
      (Variables|/Script/Engine.ProjectileMovementComponent|SetProjectileGravityScale _projectilemovement 0.0)
      (Components|Activation|Deactivate _projectilemovement)
      (Transformation|AttachActorToActor OtherActor "None" "KeepWorld" "KeepWorld" "KeepWorld" true)
      (Components|Activation|Deactivate (Variables|Default|GetParticleSystem))
      (Collision|SetCollisionEnabled (Variables|Default|GetArrowMesh) "NoCollision")
      (Variables|Default|SetHit true))))

(event EventBeginPlay
  (Utilities|FlowControl|Delay 0.1)
  (if (not (Variables|Default|GetHit))
    (Components|Activation|Activate (Variables|Default|GetParticleSystem) false)))

(event Collision|EventActorBeginOverlap
  (params (OtherActor :type Actor%20Object%20Reference)))

(event EventTick
  (params (DeltaSeconds :type Float%20%28single-precision%29)))

(fn ConstructionScript
  (bind _ammodata (Variables|Default|GetAmmoData))
  (Components|StaticMesh|SetStaticMesh (Variables|Default|GetArrowMesh) (.mesh _ammodata))
  (Variables|/Script/Engine.ProjectileMovementComponent|SetMaxSpeed (Variables|Default|GetProjectileMovement) (.maxspeed _ammodata))
  (Variables|/Script/Engine.ProjectileMovementComponent|SetInitialSpeed (Variables|Default|GetProjectileMovement) (Math|Float|MapRangeClamped (Variables|Default|GetDrawPercentage) 0.0 1.0 (.minspeed _ammodata) (.maxspeed _ammodata)))
  (Variables|/Script/Engine.ProjectileMovementComponent|SetProjectileGravityScale (Variables|Default|GetProjectileMovement) (.fallspeed _ammodata)))

(fn AddForcetoObject
  (params (Object :type Primitive%20Component%20Object%20Reference))
  (bind _projectilemovement (Variables|Default|GetProjectileMovement))
  (bind _initialspeed (Variables|/Script/Engine.ProjectileMovementComponent|GetInitialSpeed _projectilemovement))
  (bind _maxspeed (Variables|/Script/Engine.ProjectileMovementComponent|GetMaxSpeed _projectilemovement))
  (bind _returnvalue (/ _initialspeed _maxspeed))
  (Transformation|AddActorLocalOffset (* (Math|Vector|MakeVector (Variables|Default|GetMaxPenerationOffset) 0.0 0.0) _returnvalue) false false)
  (Class|PrimitiveComponent|AddForceatLocation Object (* (Transformation|GetVelocity) (* _returnvalue (Variables|Default|GetArrowMaxForce))) (Transformation|GetActorLocation) "None"))