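; Recurve bow weapon for the player character: holding fire draws the bow and releasing launches an arrow.
; While fire is held, Tick accumulates draw time and, once, socket-attaches the arrow mesh and starts hold montages on arms and bow.
; Release plays an arms montage, then spawns the arrow class, passing raw hold time as DrawPercentage.
; Equipping attaches the bow to the first-person mesh's WeaponSocket.
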(event EventBeginPlay
  (bind _arrowmesh (Variables|Default|GetArrowMesh))
  (Rendering|SetVisibility _arrowmesh true false)
  (Components|StaticMesh|SetStaticMesh _arrowmesh (.mesh (Utilities|GetClassDefaults (Variables|Default|GetArrowClass))))
  (bind _returnvalue (Transformation|AttachComponentToComponent (Variables|Default|GetArrowMesh) (Variables|Default|GetFirstPersonMesh) "ArrowSocket" "SnapToTarget" "KeepRelative" "KeepRelative" true))
  (if _returnvalue
    _))

(event Collision|EventActorBeginOverlap
  (params (OtherActor :type Actor%20Object%20Reference)))

(event EventTick
  (params (DeltaSeconds :type Float%20%28single-precision%29))
  (bind _arrowmesh (Variables|Default|GetArrowMesh))
  (bind _firstpersonmesh (Variables|Default|GetFirstPersonMesh))
  (bind _weaponmesh (Variables|Default|GetWeaponMesh))
  (bind _returnvalue (Components|SkeletalMesh|GetAnimInstance _firstpersonmesh))
  (bind _returnvalue_2 (Components|SkeletalMesh|GetAnimInstance _weaponmesh))
  (if (Variables|Default|GetIsHolding)
    (Variables|Default|SetTenseTime (+ DeltaSeconds (Variables|Default|GetTenseTime)))
    (if (not (Variables|Default|GetStartedHolding))
      (if (Transformation|DoesSocketExist (Variables|Default|GetFirstPersonMesh) "ArrowSocket")
        (Rendering|SetVisibility _arrowmesh true false)
        (Components|StaticMesh|SetStaticMesh _arrowmesh (.mesh (Utilities|GetClassDefaults (Variables|Default|GetArrowClass))))
        (Transformation|AttachComponentToComponent (Variables|Default|GetArrowMesh) (Variables|Default|GetFirstPersonMesh) "ArrowSocket" "SnapToTarget" "KeepRelative" "KeepRelative" true)
        (Animation|Montage|PlayMontage _firstpersonmesh (Variables|Default|GetArmsHoldMontage) 1.0 0.0 "LoadToHold"
          (:then
            (Variables|Default|SetIdleToAdsArmsLength (Animation|Montage|MontageGetPosition _returnvalue (Animation|Montage|GetCurrentActiveMontage _returnvalue)))
            (Animation|Montage|PlayMontage _weaponmesh (Variables|Default|GetBowHoldMontage) 1.0 0.0 "Shoot"
              (:then
                (Variables|Default|SetIdle%20to%20ADS%20weapons%20TIme (Animation|Montage|MontageGetPosition _returnvalue_2 (Animation|Montage|GetCurrentActiveMontage _returnvalue_2)))
                (Variables|Default|SetStartedHolding true)))))
        (else
          (Development|PrintString "No Socket"))))))

(event EventOnFire
  (Variables|Default|SetIsHolding true))

(event EventOnFireStopped
  (bind _arrow (Variables|Default|GetArrow))
  (Variables|Default|SetStartedHolding false)
  (Variables|Default|SetIsHolding false)
  (Animation|Montage|MontageStop (Components|SkeletalMesh|GetAnimInstance (Variables|Default|GetWeaponMesh)) 0.0 (Variables|Default|GetBowHoldMontage))
  (Rendering|SetVisibility (Variables|Default|GetArrowMesh) false false)
  (Animation|Montage|PlayMontage (Variables|Default|GetFirstPersonMesh) "/Game/Users/Aadit/PlayerCharacters/Arms/Animations/ANIM_FP_Arms_LongBow_IdleToADS_Montage.ANIM_FP_Arms_LongBow_IdleToADS_Montage" 1.0 0.0 "StartLoad"
    (:then
      (Rendering|SetVisibility (Variables|Default|GetArrowMesh) true false)
      (bind _asbase_game_character (Utilities|Casting|CastToBaseGameCharacter (Components|GetOwner)))
      (Game|SpawnActorfromClass (Variables|Default|GetArrowClass) (Math|Transform|MakeTransform (Transformation|GetWorldLocation _arrow) (Transformation|GetWorldRotation _arrow)) "AdjustIfPossibleButAlwaysSpawn" self (Variables|Default|GetTenseTime) _asbase_game_character)
      (Audio|PlaySound2D "/Game/Users/Aadit/AudioEvents/Bow_Launch_Arrow.Bow_Launch_Arrow")
      (Variables|Default|SetTenseTime 0.0))))

(event EventOnEquipped
  (CallFunction|SetUpBows))

(fn ConstructionScript
  (bind _asbp_player_game_character (Utilities|Casting|CastToBP_PlayerGameCharacter (Components|GetOwner)))
  (Variables|Default|SetFirstPersonMesh (Variables|/Script/Vaudeville.PlayerGameCharacter|GetFirstPersonMesh _asbp_player_game_character)))

(fn SetUpBows
  (bind _asbp_player_game_character (Utilities|Casting|CastToBP_PlayerGameCharacter (Components|GetOwner)))
  (Transformation|SetActorTransform self (Transformation|GetSocketTransform (Variables|/Script/Vaudeville.PlayerGameCharacter|GetFirstPersonMesh _asbp_player_game_character) "WeaponSocket" "RTS_World") false true)
  (Transformation|AttachComponentToComponent self (Variables|/Script/Vaudeville.PlayerGameCharacter|GetFirstPersonMesh _asbp_player_game_character) "WeaponSocket" "KeepWorld" "KeepWorld" "KeepWorld" true))